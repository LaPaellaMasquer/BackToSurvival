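; BPRobotSpider is a robot spider character with two action components and animated reactions to being hit and dying.
; On BeginPlay it assigns the components to its Action1 and Action2 slots, gives each the SpiderMech mesh, and binds to the hit and death events of its life object.
; Hit and death play montages on that mesh, and death also deactivates the capsule.
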(event `self.ReceiveBeginPlay`
  (bind _bpspideraction1component (`self.BPSpiderAction1Component`))
  (bind _bpspideraction2component (`self.BPSpiderAction2Component`))
  (bind _spidermech (`self.SpiderMech`))
  (set `self.action1` _bpspideraction1component)
  (set `XScanActionComponent.ownerMesh` _spidermech _bpspideraction1component)
  (set `self.action2` _bpspideraction2component)
  (set `XScanActionComponent.ownerMesh` _spidermech _bpspideraction2component)
  (bind _returnvalue (`self.GetLife`))
  (add `LifeComponent.OnHit` _returnvalue (delegate `HitAnimation`))
  (add `LifeComponent.OnDeath` _returnvalue (delegate `DeathAnimation`)))

(event `HitAnimation`
  (`|PlayMontage` (`self.SpiderMech`) "/Game/Blueprints/Spider/BPSpiderHitMontage.BPSpiderHitMontage" 1.0 0.0 "Hit"))

(event `DeathAnimation`
  (`|PlayMontage` (`self.SpiderMech`) "/Game/Blueprints/Spider/BPSpiderDeathMontage.BPSpiderDeathMontage" 1.0 0.0 "Death"
    (:`then`
      (`ActorComponent.SetActive` (`self.Capsule`) false false))))

(fn `UserConstructionScript`)