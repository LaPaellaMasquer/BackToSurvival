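; BPDog is a dog actor that wires up two action components and animated reactions to being hit and dying.
; On BeginPlay it fills its two action slots with BPDogAction1 and BPDogAction2, giving each the Dog mesh as owner mesh.
; It binds to the hit and death events from GetLife to play the matching montages on that mesh.
; The death handler also deactivates the Capsule component.
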(event `self.ReceiveBeginPlay`
  (bind _dog (`self.Dog`))
  (bind _bpdogaction1 (`self.BPDogAction1`))
  (bind _bpdogaction2 (`self.BPDogAction2`))
  (set `self.action1` _bpdogaction1)
  (set `XScanActionComponent.ownerMesh` _dog _bpdogaction1)
  (set `self.action2` _bpdogaction2)
  (set `XScanActionComponent.ownerMesh` _dog _bpdogaction2)
  (bind _returnvalue (`self.GetLife`))
  (add `LifeComponent.OnHit` _returnvalue (delegate `HitAnimation`))
  (add `LifeComponent.OnDeath` _returnvalue (delegate `DeathAnimation`)))

(event `HitAnimation`
  (`|PlayMontage` (`self.Dog`) "/Game/Blueprints/Dog/BPDogHitMontage.BPDogHitMontage" 1.0 0.0 "Hit"))

(event `DeathAnimation`
  (`|PlayMontage` (`self.Dog`) "/Game/Blueprints/Dog/BPDogDeathMontage.BPDogDeathMontage" 1.0 0.0 "Death"
    (:`then`
      (`ActorComponent.SetActive` (`self.Capsule`) false false))))

(fn `UserConstructionScript`)