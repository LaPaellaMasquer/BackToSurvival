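; Behavior tree task that moves an enemy pawn and plays its Action1 on a valid target.
; It scans actors within blue movement range plus action range, filtering by the action's life and team check.
; Each match triggers an AIMoveTo toward normalized direction plus range, without adding pawn position, and the scan then calls FinishExecute(false) immediately.
; On move success, it faces the target, sets the goal, animates and spends all current PA.
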(event `self.ReceiveExecuteAI`
  (params (OwnerController :type "AIController Object Reference") (ControlledPawn :type "Pawn Object Reference"))
  (bind _asennemy_aicontroller (cast `EnnemyAIController` OwnerController)
    (:`then`
      (bind _ascharacter_pawn (cast `CharacterPawn` ControlledPawn)
        (:`then`
          (set `self.character Pawn` _ascharacter_pawn)
          (`self.Find Action Target` _asennemy_aicontroller (`CharacterPawn.action1` _ascharacter_pawn)))
        (:`CastFailed`
          (`self.FinishAbort`))))
    (:`CastFailed`
      (`self.FinishAbort`))))

(event `Move`
  (params (Location :type "Vector Structure"))
  (bind _character_pawn (`self.character Pawn`))
  (`self.LookAt` _character_pawn Location)
  (`|AIMoveTo` _character_pawn Location null -1.0
    (:`OnSuccess`
      (bind _success (`self.Play Action`))
      (`self.FinishExecute` _success))))

(fn `Find Action Target`
  (params (controller :type "EnnemyAIController Object Reference") (action :type "ActionComponentBase Object Reference"))
  (bind _character_pawn (`self.character Pawn`))
  (bind _returnvalue (`ActionComponentBase.GetRange` action))
  (bind _returnvalue_2 (`CharacterPawn.GetMovement` _character_pawn))
  (bind _returnvalue_3 (`MoveComponent.GetBlueRange` _returnvalue_2))
  (bind _returnvalue_4 (`EnnemyAIController.GetActorsInSightRadius` controller (+ _returnvalue_3 _returnvalue)))
  (for _array_element _returnvalue_4
    (bind _ascharacter_pawn (cast `CharacterPawn` _array_element))
    (bind _returnvalue_5 (`CharacterPawn.GetLife` _ascharacter_pawn))
    (bind _returnvalue_6 (`LifeComponent.GetPv` _returnvalue_5))
    (bind _returnvalue_7 (`LifeComponent.GetMaxPv` _returnvalue_5))
    (bind _returnvalue_8 (`ActionComponentBase.isEffectOnOpponent` action (`KismetMathLibrary.FTrunc` _returnvalue_6) (`KismetMathLibrary.FTrunc` _returnvalue_7) (`CharacterPawn.tag` _ascharacter_pawn) (`CharacterPawn.tag` _character_pawn)))
    (if _returnvalue_8
      (set `self.Target` _ascharacter_pawn)
      (`self.Move` (+ (`KismetMathLibrary.Normal` (- (`Actor.K2_GetActorLocation` _ascharacter_pawn) (`Actor.K2_GetActorLocation` _character_pawn))) (`KismetMathLibrary.MakeVector` _returnvalue _returnvalue _returnvalue)))))
  (`self.FinishExecute` false))

(fn `LookAt`
  (params (Character :type "CharacterPawn Object Reference") (Target :type "Vector Structure"))
  (`Actor.K2_SetActorRotation` Character (`KismetMathLibrary.FindLookAtRotation` (`Actor.K2_GetActorLocation` Character) Target) false))

(fn `Play Action`
  (returns (Success :type Boolean))
  (bind _target (`self.Target`))
  (bind _character_pawn (`self.character Pawn`))
  (bind _returnvalue (`Actor.K2_GetActorLocation` _target))
  (bind _action1 (`CharacterPawn.action1` _character_pawn))
  (`self.LookAt` null _returnvalue)
  (bind _returnvalue_2 (`ActionComponentBase.SetGoal` _action1 (`GameplayStatics.MakeHitResult` false false 0.0 0.0 _returnvalue (0.0 0.0 0.0) (0.0 0.0 1.0) (0.0 0.0 1.0) null _target)))
  (if _returnvalue_2
    (`ActionComponentBase.PlayAnim` _action1)
    (bind _returnvalue_3 (`CharacterPawn.GetPA` _character_pawn))
    (bind _returnvalue_4 (`PAComponent.GetCurrentPA` _returnvalue_3))
    (`PAComponent.DecreasePA` _returnvalue_3 (`KismetMathLibrary.Conv_ByteToInt` _returnvalue_4))
    (return true)
    (else
      (return false))))