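; Behavior tree task that moves an AI CharacterPawn to a random reachable point within its movement's orange range.
; It rotates the pawn toward that point, runs AIMoveTo, and on success spends all current PA before finishing.
; Failed casts abort the task, but a failed move has no handler.
; A loop targeting a differently tagged pawn in sight is disconnected, so the sight query result goes unused.
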(event `self.ReceiveExecuteAI`
  (params (OwnerController :type "AIController Object Reference") (ControlledPawn :type "Pawn Object Reference"))
  (bind _target (`self.target`))
  (bind _ascharacter_pawn (cast `CharacterPawn` ControlledPawn)
    (:`then`
      (bind _asennemy_aicontroller (cast `EnnemyAIController` OwnerController)
        (:`then`
          (bind _returnvalue (`CharacterPawn.GetMovement` _ascharacter_pawn))
          (bind _returnvalue_2 (`MoveComponent.GetOrangeRange` _returnvalue))
          (bind _returnvalue_3 (`EnnemyAIController.GetActorsInSightRadius` _asennemy_aicontroller _returnvalue_2))
          (set `self.target` (`NavigationSystemV1.K2_GetRandomReachablePointInRadius` (`Actor.K2_GetActorLocation` _ascharacter_pawn) _returnvalue_2 null null))
          (`self.LookAt` _ascharacter_pawn _target)
          (`|AIMoveTo` OwnerController ControlledPawn _target null 5.0 true
            (:`OnSuccess`
              (bind _returnvalue_4 (`CharacterPawn.GetPA` _ascharacter_pawn))
              (bind _returnvalue_5 (`PAComponent.GetCurrentPA` _returnvalue_4))
              (`PAComponent.DecreasePA` _returnvalue_4 (`KismetMathLibrary.Conv_ByteToInt` _returnvalue_5))
              (`self.FinishExecute` true))))
        (:`CastFailed`
          (`self.FinishAbort`))))
    (:`CastFailed`
      (`self.FinishAbort`))))

(fn `LookAt`
  (params (Character :type "CharacterPawn Object Reference") (Target :type "Vector Structure"))
  (`Actor.K2_SetActorRotation` Character (`KismetMathLibrary.FindLookAtRotation` (`Actor.K2_GetActorLocation` Character) Target) false))