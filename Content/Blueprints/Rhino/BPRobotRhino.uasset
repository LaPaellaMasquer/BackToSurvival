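; Rhino robot Blueprint that wires up the robot's two actions and its hit and death animations.
; On BeginPlay it assigns its two rhino action components to the Action1 and Action2 slots and hands each the Behemoth mesh.
; It also binds to the life object's OnHit and OnDeath events to play montages on that mesh.
; Death also deactivates the capsule and box as soon as the montage starts, without waiting for completion.
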(event `self.ReceiveBeginPlay`
  (bind _behemoth_sketchfab (`self.BEHEMOTH_SKETCHFAB`))
  (bind _bprhinoaction1 (`self.BPRhinoAction1`))
  (bind _bprhinoaction2 (`self.BPRhinoAction2`))
  (set `self.action1` _bprhinoaction1)
  (set `XScanActionComponent.ownerMesh` _behemoth_sketchfab _bprhinoaction1)
  (set `self.action2` _bprhinoaction2)
  (set `XScanActionComponent.ownerMesh` _behemoth_sketchfab _bprhinoaction2)
  (bind _returnvalue (`self.GetLife`))
  (add `LifeComponent.OnHit` _returnvalue (delegate `HitAnimation`))
  (add `LifeComponent.OnDeath` _returnvalue (delegate `DeathAnimation`)))

(event `HitAnimation`
  (`|PlayMontage` (`self.BEHEMOTH_SKETCHFAB`) "/Game/Blueprints/Rhino/BPRobotRhinoHitMontage.BPRobotRhinoHitMontage" 1.0 0.0 "Hit"))

(event `DeathAnimation`
  (`|PlayMontage` (`self.BEHEMOTH_SKETCHFAB`) "/Game/Blueprints/Rhino/BPRobotRhinoDeathMontage.BPRobotRhinoDeathMontage" 1.0 0.0 "Death"
    (:`then`
      (`ActorComponent.SetActive` (`self.Capsule`) false false)
      (`ActorComponent.SetActive` (`self.Box`) false false))))

(fn `UserConstructionScript`)