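; Bubble robot Blueprint that sets up the character's two actions and its hit and death animation reactions.
; On BeginPlay it assigns two bubble action objects as Action1 and Action2, handing each the robot's skeletal mesh.
; It binds to the hit and death events of its Life object to play the matching montages.
; Death also deactivates the capsule as soon as the montage starts, without waiting for completion.
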(event `self.ReceiveBeginPlay`
  (bind _robotbubble (`self.RobotBubble`))
  (bind _bpbubbleaction2 (`self.BPBubbleAction2`))
  (bind _bpbubbleacion1 (`self.BPBubbleAcion1`))
  (set `self.action1` _bpbubbleacion1)
  (set `XScanActionComponent.ownerMesh` _robotbubble _bpbubbleacion1)
  (set `self.action2` _bpbubbleaction2)
  (set `XScanActionComponent.ownerMesh` _robotbubble _bpbubbleaction2)
  (bind _returnvalue (`self.GetLife`))
  (add `LifeComponent.OnHit` _returnvalue (delegate `HitAnimation`))
  (add `LifeComponent.OnDeath` _returnvalue (delegate `DeathAnimation`)))

(event `HitAnimation`
  (`|PlayMontage` (`self.RobotBubble`) "/Game/Blueprints/Bubble/BPBubbleHitAnimMontage.BPBubbleHitAnimMontage" 1.0 0.0 "Hit"))

(event `DeathAnimation`
  (`|PlayMontage` (`self.RobotBubble`) "/Game/Blueprints/Bubble/BPBubbleDeathAnimMontage.BPBubbleDeathAnimMontage" 1.0 0.0 "Death"
    (:`then`
      (`ActorComponent.SetActive` (`self.Capsule`) false false))))

(event `self.ReceiveTick`
  (params (DeltaSeconds :type "Float (single-precision)")))

(fn `UserConstructionScript`)