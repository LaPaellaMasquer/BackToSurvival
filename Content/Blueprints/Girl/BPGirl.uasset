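; BPGirl is the girl character Blueprint, wiring up her two actions and her damage reactions.
; On BeginPlay it assigns its two action components, handing each the Girl skeletal mesh as owner.
; It binds its Life's hit and death events to montage playback on that mesh.
; The death montage's Then output also deactivates the capsule.
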(event `self.ReceiveBeginPlay`
  (bind _girl (`self.Girl`))
  (bind _bpgirlaction2 (`self.BPGirlAction2`))
  (bind _bpgirlaction1 (`self.BPGirlAction1`))
  (set `self.action1` _bpgirlaction1)
  (set `XScanActionComponent.ownerMesh` _girl _bpgirlaction1)
  (set `self.action2` _bpgirlaction2)
  (set `XScanActionComponent.ownerMesh` _girl _bpgirlaction2)
  (bind _returnvalue (`self.GetLife`))
  (add `LifeComponent.OnHit` _returnvalue (delegate `HitAnimation`))
  (add `LifeComponent.OnDeath` _returnvalue (delegate `DeathAnimation`)))

(event `HitAnimation`
  (`|PlayMontage` (`self.Girl`) "/Game/Blueprints/Girl/BPGirlHitMontage.BPGirlHitMontage" 1.0 0.0 "Hit"))

(event `DeathAnimation`
  (`|PlayMontage` (`self.Girl`) "/Game/Blueprints/Girl/BPGirlDeathMontage.BPGirlDeathMontage" 1.0 0.0 "Death"
    (:`then`
      (`ActorComponent.SetActive` (`self.Capsule1`) false false))))

(fn `UserConstructionScript`)