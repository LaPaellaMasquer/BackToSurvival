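; BPLumberjack is the lumberjack character Blueprint, wiring up its actions and its reactions to damage.
; On BeginPlay it assigns two lumberjack action objects to its action slots and hands each the LumberJack mesh as owner mesh.
; It also binds the Life object's hit and death events to montages on that mesh, with death also deactivating the capsule once the montage call is issued.
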(event `self.ReceiveBeginPlay`
  (bind _lumberjack (`self.LumberJack`))
  (bind _bplumberjackaction1 (`self.BPLumberjackAction1`))
  (bind _bplumberjackaction2 (`self.BPLumberjackAction2`))
  (set `self.action1` _bplumberjackaction1)
  (set `XScanActionComponent.ownerMesh` _lumberjack _bplumberjackaction1)
  (set `self.action2` _bplumberjackaction2)
  (set `XScanActionComponent.ownerMesh` _lumberjack _bplumberjackaction2)
  (bind _returnvalue (`self.GetLife`))
  (add `LifeComponent.OnHit` _returnvalue (delegate `HitAnimation`))
  (add `LifeComponent.OnDeath` _returnvalue (delegate `DeathAnimation`)))

(event `HitAnimation`
  (`|PlayMontage` (`self.LumberJack`) "/Game/Blueprints/LumberJack/BPLumberjackHitMontage.BPLumberjackHitMontage" 1.0 0.0 "Hit"))

(event `DeathAnimation`
  (`|PlayMontage` (`self.LumberJack`) "/Game/Blueprints/LumberJack/BPLumberjackDeathMontage.BPLumberjackDeathMontage" 1.0 0.0 "Death"
    (:`then`
      (`ActorComponent.SetActive` (`self.Capsule`) false false))))

(fn `UserConstructionScript`)